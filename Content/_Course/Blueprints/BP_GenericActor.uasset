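; BP_GenericActor is a course actor that randomly changes its point light's intensity and colour every two seconds from BeginPlay.
; A self-recalling event calls FnGetRandomValue, applies the returned intensity, prints the returned name and delays.
; The function maps a random MyArray name to an intensity, ignoring its InputArray parameter, and sets a random ColourList colour itself.
; A while-loop print and a struct-driven colour switch are disconnected and never run.
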(event Custom|evGetRandomValue
  (bind (_outputstring _new_intensity) (CallFunction|FnGetRandomValue (Variables|Default|GetMyArray)))
  (Rendering|Components|Light|SetIntensity (Variables|Default|GetPointLight) _new_intensity)
  (Development|PrintString _outputstring true true "(R=0.000000,G=0.660000,B=1.000000,A=1.000000)" 5.0)
  (Utilities|FlowControl|Delay 2.0)
  (CallFunction|EvGetRandomValue))

(event EventBeginPlay
  (CallFunction|EvGetRandomValue))

(event EventTick
  (params (DeltaSeconds :type Float%20%28single-precision%29)))

(fn ConstructionScript)

(fn FnGetRandomValue
  (params (InputArray :type Array%20of%20Strings))
  (Utilities|FlowControl|Sequence
    (:then_0
      (switch string (.OutItem (Utilities|Array|Random (Variables|Default|GetMyArray)))
        (:Hasan
          (LocalVariables|SetStringSelection "Hasan")
          (LocalVariables|SetLight%20Intensity 4e+03))
        (:Ahmed
          (LocalVariables|SetStringSelection "Ahmed")
          (LocalVariables|SetLight%20Intensity 3e+04))
        (:Abdalla
          (LocalVariables|SetStringSelection "Abdalla")
          (LocalVariables|SetLight%20Intensity 6e+04))
        (:Kheir
          (LocalVariables|SetStringSelection "Kheir")
          (LocalVariables|SetLight%20Intensity 1e+05))))
    (:then_1
      (Rendering|Components|Light|SetLightColor (Variables|Default|GetPointLight) (.OutItem (Utilities|Array|Random (Variables|Default|GetColour%20List))) true))
    (:then_2
      (return (LocalVariables|GetStringSelection) (LocalVariables|GetLight%20Intensity)))))