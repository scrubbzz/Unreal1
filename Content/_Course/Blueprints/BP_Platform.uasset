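; BP_Platform is a platform actor that slides its Cube component one way from its starting relative location to EndLocation.
; BeginPlay stores the start location, then Tick lerps between the two points without sweep.
; Alpha rises by a fixed, frame-rate-dependent step each tick and is clamped at one, so the cube stops at the end.
; An unconnected VInterpTo node is left unused.
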(event EventBeginPlay
  (Variables|Default|SetStartLocation (Variables|/Script/Engine.SceneComponent|GetRelativeLocation (Variables|Default|GetCube))))

(event EventTick
  (params (DeltaSeconds :type Float%20%28single-precision%29))
  (Transformation|SetRelativeLocation (Variables|Default|GetCube) (Math|Vector|Lerp(Vector) (Variables|Default|GetStartLocation) (Variables|Default|GetEndLocation) (Variables|Default|GetAlpha)) false false)
  (Variables|Default|SetAlpha (Math|Float|Clamp(Float) (+ (Variables|Default|GetAlpha) 0.01))))

(fn ConstructionScript)